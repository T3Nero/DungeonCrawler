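; Wave manager that spawns enemies and an optional pickup per wave from WaveDataMap, keyed by wave index.
; Enemies appear at random points within SpawnArea at a fixed height, receive a manager reference and are tracked in ActiveEnemies; pickups spawn at PickUpPos.
; When EnemyDefeated empties that list, it updates the wave text and starts the next wave after a random delay.
; Once all waves are cleared, it reloads the current level.
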(event Custom|SpawnWave
  (bind _wavedatamap (Variables|Default|GetWaveDataMap))
  (bind _currentwaveindex (Variables|Default|GetCurrentWaveIndex))
  (bind (_value _returnvalue) (Utilities|Map|Find _wavedatamap _currentwaveindex))
  (bind (_enemies _pickup) (Utilities|Struct|BreakS_WaveData _value))
  (if _returnvalue
    (for _array_element _enemies
      (CallFunction|SpawnEnemy _array_element))
    (if (Utilities|IsValidClass _pickup)
      (CallFunction|SpawnPickUp _pickup))))

(event Custom|SpawnNextWave
  (Math|Integer|IncrementInt (Variables|Default|GetCurrentWaveIndex)
    (:%20%20
      (if (>= (Utilities|Map|Length (Variables|Default|GetWaveDataMap)) (Variables|Default|GetCurrentWaveIndex))
        (Default|CallUpdateWaveText (Variables|Default|GetCurrentWaveIndex) false)
        (Utilities|FlowControl|Delay (Math|Random|RandomFloatinRange 1.0 2.0))
        (CallFunction|SpawnWave)
        (else
          (Default|CallUpdateWaveText 0 true)
          (Utilities|FlowControl|Delay 2.0)
          (bind _returnvalue (Game|GetCurrentLevelName true))
          (Game|OpenLevel(byName) (Utilities|String|StringToName _returnvalue)))))))

(event EventBeginPlay
  (Utilities|FlowControl|Delay (Math|Random|RandomFloatinRange 0.5 1.0))
  (CallFunction|SpawnWave))

(fn ConstructionScript)

(fn SpawnEnemy
  (params (Enemy :type BP%20Enemy%20Base%20Class%20Reference))
  (bind _spawnarea (Variables|Default|GetSpawnArea))
  (bind (_origin _boxextent) (Collision|GetComponentBounds _spawnarea))
  (bind _returnvalue (Math|Random|RandomPointinBoundingBox _origin _boxextent))
  (bind _returnvalue_2 (Game|SpawnActorfromClass Enemy (Math|Transform|MakeTransform (Math|Vector|MakeVector (.x _returnvalue) (.y _returnvalue) (LocalVariables|GetSpawnHeight)) "0, 0, 0" "1.000000,1.000000,1.000000") "AlwaysSpawn" "MultiplyWithRoot" 0 self 0))
  (Utilities|Array|Add (Variables|Default|GetActiveEnemies) _returnvalue_2))

(fn EnemyDefeated
  (params (Enemy :type BP%20Enemy%20Base%20Object%20Reference%20%28by%20ref%29))
  (bind _activeenemies (Variables|Default|GetActiveEnemies))
  (Utilities|Array|RemoveItem _activeenemies Enemy)
  (if (<= (Utilities|Array|Length _activeenemies) 0)
    (CallFunction|SpawnNextWave)))

(fn SpawnPickUp
  (params (PickUp :type Actor%20Class%20Reference))
  (Game|SpawnActorfromClass PickUp (Math|Transform|MakeTransform (Transformation|GetWorldLocation (Variables|Default|GetPickUpPos)) "0, 0, 0" "1.000000,1.000000,1.000000") "AlwaysSpawn" "MultiplyWithRoot" 0 0))