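; BP_EnemyBase is a base enemy character that chases, deals contact damage, gets stunned and dies.
; ChasePlayer feeds movement input along a supplied direction while the enemy is alive and unstunned.
; Overlap with a Player-tagged actor triggers hit stop, with damage applied only through the player's HitDetectBox.
; HandleHitStates extends the parent with a retriggerable stun, and on death spawns a skull explosion before destroying the actor.
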(event OnComponentBeginOverlap(HitDetectBox)
  (params (OverlappedComponent :type Primitive%20Component%20Object%20Reference) (OtherActor :type Actor%20Object%20Reference) (OtherComp :type Primitive%20Component%20Object%20Reference) (OtherBodyIndex :type Integer) (bFromSweep :type Boolean) (SweepResult :type Hit%20Result%20Structure%20%28by%20ref%29))
  (if (Default|IsAlive (Variables|Default|GetHealthComponent))
    (if (Actor|ActorHasTag OtherActor "Player")
      (CallFunction|HitStop)
      (bind _asbp_player_character (Utilities|Casting|CastToBP_PlayerCharacter OtherActor))
      (if (== OtherComp (Variables|/Game/Blueprints/Characters/BP_BaseCharacter.BP_BaseCharacter_C|GetHitDetectBox _asbp_player_character))
        (Game|Damage|ApplyDamage OtherActor (Variables|Combat|GetBase%20Damage) 0 self)))))

(event Custom|ChasePlayer
  (params (WorldDirection :type Vector))
  (if (and (Default|IsAlive (Variables|Default|GetHealthComponent)) (not (Variables|Default|GetIsStunned)))
    (Pawn|Input|AddMovementInput WorldDirection 1.0 false)))

(event Custom|HandleStun
  (Variables|Default|SetIsStunned true)
  (Utilities|FlowControl|RetriggerableDelay (Variables|Default|GetStunDuration))
  (Variables|Default|SetIsStunned false))

(event Custom|HandleDeath
  (Game|SpawnActorfromClass "/Game/Blueprints/VFX/BP_VFX_SkullExplosion.BP_VFX_SkullExplosion_C" (Math|Transform|MakeTransform (Transformation|GetActorLocation) "0, 0, 0" "1.000000,1.000000,1.000000") "AlwaysSpawn" "MultiplyWithRoot" 0 0)
  (Actor|DestroyActor))

(event EventBeginPlay
  (|CallParentFunction)
  (Variables|/Script/Engine.CharacterMovementComponent|SetMaxWalkSpeed (Variables|Character|GetCharacterMovement) (Variables|Movement|GetWalkSpeed)))

(event Collision|EventActorBeginOverlap
  (params (OtherActor :type Actor%20Object%20Reference))
  (|CallParentFunction OtherActor) ; This node is disabled and will not be called.\nDrag off pins to build functionality.
)

(event EventTick
  (params (DeltaSeconds :type Float%20%28single-precision%29))
  (|CallParentFunction DeltaSeconds) ; This node is disabled and will not be called.\nDrag off pins to build functionality.
)

(event EventHandleHitStates
  (|CallParentFunction)
  (CallFunction|HandleStun)
  (if (not (Default|IsAlive (Variables|Default|GetHealthComponent)))
    (CallFunction|HandleDeath)))

(fn ConstructionScript
  (|CallParentFunction))