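; Base character Blueprint that handles taking damage with a hit reaction, knockback and death.
; AnyDamage lowers HealthComponent health, starts knockback and plays a PaperZD hit animation override, setting IsStunned until it completes or cancels.
; On completion or cancel, a character without health jumps to the death animation node.
; Knockback uses a timeline to push velocity away from the attacker, clamping its delta-time-scaled size for consistency across frame rates.
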(event Custom|Knockback
  (params (Attacker :type Actor%20Object%20Reference))
  (Variables|Default|SetKnockbackDirection (Math|Vector|GetForwardVector (Math|Rotator|FindLookatRotation (Transformation|GetActorLocation Attacker) (Transformation|GetActorLocation))))
  (Components|Timeline|SetPlayRate (Variables|Default|GetKnockbackTimeline) 5.0)
  (Timeline|KnockbackTimeline PlayFromStart
    (:Update
      ;[1 1 1] Knockback Force of 300 000 to simulate a max fps of 300: Clamp Max Kb Dist to maintain Kb velocity over varied fps
      (Variables|/Script/Engine.MovementComponent|SetVelocity (Variables|Character|GetCharacterMovement) (Math|Vector|VectorClampSizeMax (* (Variables|Default|GetKnockbackDirection) (Variables|Default|GetKnockbackForce) (Utilities|Time|GetWorldDeltaSeconds)) (Variables|Default|GetMaxKnockbackDistance))))))

(event EventBeginPlay)

(event Collision|EventActorBeginOverlap
  (params (OtherActor :type Actor%20Object%20Reference)))

(event EventTick
  (params (DeltaSeconds :type Float%20%28single-precision%29)))

(event Game|Damage|EventAnyDamage
  (params (Damage :type Float%20%28single-precision%29) (DamageType :type Damage%20Type%20Object%20Reference) (InstigatedBy :type Controller%20Object%20Reference) (DamageCauser :type Actor%20Object%20Reference))
  (bind _healthcomponent (Variables|Default|GetHealthComponent))
  (Variables|Default|SetDamageTaken Damage)
  (if (Default|IsAlive _healthcomponent)
    (Default|DecreaseHealth _healthcomponent (Variables|Default|GetDamageTaken))
    (CallFunction|Knockback DamageCauser)
    (|PlayAnimationOverridewithCallbacks (Variables|Default|GetAnimInstance) (Variables|Default|GetGetHitAnim) "DefaultSlot" 1.0 0.0
      (:then
        (Variables|Default|SetIsStunned true))
      (:OnCompleted
        (Variables|Default|SetIsStunned false :!label _label)
        (if (not (Default|IsAlive (Variables|Default|GetHealthComponent)))
          (Class|PaperZDAnimInstance|JumptoNode (Variables|Default|GetAnimInstance) "DeadJump" "None")))
      (:OnCancelled
        (goto _label)))))

(fn ConstructionScript)