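; Player character for a sprite-based dungeon game, with movement, sword and bow attacks, a heart-piece health HUD, healing and death.
; Enhanced Input actions pass a CanAct gate, and animation override callbacks set and clear the attacking and stunned states.
; Separate functions damage enemies overlapping the HitBox or spawn arrows.
; Hits update the HUD, request invincibility and play a stun animation, then start sprite flicker or, on death, reload the level.
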(event Input|EnhancedActionEvents|EnhancedInputActionIA_Move
  (params (ActionValue :type Vector%202D%20Structure) (ElapsedSeconds :type Float%20%28double-precision%29) (TriggeredSeconds :type Float%20%28double-precision%29) (InputAction :type Input%20Action%20Object%20Reference :default "/Game/Input/Actions/IA_Move.IA_Move"))
  (bind (_x _y) (Math|Vector2D|BreakVector2D ActionValue))
  (if (CallFunction|CanAct)
    (Pawn|Input|AddMovementInput "1.000000,0.000000,0.000000" _x false)
    (Pawn|Input|AddMovementInput "0.000000,1.000000,0.000000" _y false)))

(event Input|EnhancedActionEvents|EnhancedInputActionIA_Exit
  (params (ActionValue :type Boolean) (ElapsedSeconds :type Float%20%28double-precision%29) (TriggeredSeconds :type Float%20%28double-precision%29) (InputAction :type Input%20Action%20Object%20Reference :default "/Game/Input/Actions/IA_Exit.IA_Exit"))
  (:Started
    (Game|QuitGame 0 "Quit" false)))

(event Input|EnhancedActionEvents|EnhancedInputActionIA_Attack
  (params (ActionValue :type Boolean) (ElapsedSeconds :type Float%20%28double-precision%29) (TriggeredSeconds :type Float%20%28double-precision%29) (InputAction :type Input%20Action%20Object%20Reference :default "/Game/Input/Actions/IA_Attack.IA_Attack"))
  (:Ongoing
    (if (CallFunction|CanAct)
      (CallFunction|HitStop)
      (|PlayAnimationOverridewithCallbacks (Variables|Default|GetAnimInstance) "/Game/Blueprints/Characters/Player/AnimSequences/Attack.Attack" "DefaultSlot" (Variables|Default|GetAttackSpeed) 0.0
        (:then
          (Variables|Default|SetIsAttacking true))
        (:OnCompleted
          (Variables|Default|SetIsAttacking false :!label _label))
        (:OnCancelled
          (goto _label))))))

(event Input|EnhancedActionEvents|EnhancedInputActionIA_BowAttack
  (params (ActionValue :type Boolean) (ElapsedSeconds :type Float%20%28double-precision%29) (TriggeredSeconds :type Float%20%28double-precision%29) (InputAction :type Input%20Action%20Object%20Reference :default "/Game/Input/Actions/IA_BowAttack.IA_BowAttack"))
  (:Ongoing
    (if (and (CallFunction|CanAct) (Variables|Default|GetBowEquipped))
      (CallFunction|HitStop)
      (|PlayAnimationOverridewithCallbacks (Variables|Default|GetAnimInstance) "/Game/Blueprints/Characters/Player/AnimSequences/Bow.Bow" "DefaultSlot" 1.0 0.0
        (:then
          (Variables|Default|SetIsAttacking true))
        (:OnCompleted
          (Variables|Default|SetIsAttacking false :!label _label))
        (:OnCancelled
          (goto _label))))))

(event EventBeginPlay
  (|CallParentFunction)
  (Utilities|FlowControl|Sequence
    (:then_0
      (Class|WidgetBlueprintLibrary|SetFocustoGameViewport)
      (Input|AddMappingContext (PlayerController|LocalPlayerSubsystems|GetEnhancedInputLocalPlayerSubsystem (Game|GetPlayerController 0)) "/Game/Input/IMC_Dungeon.IMC_Dungeon" 0 "(bIgnoreAllPressedKeysUntilRelease=True,bForceImmediately=False,bNotifyUserSettings=False)")
      (Transformation|SetWorldLocation (Variables|Default|GetSpringArm) (Transformation|GetActorLocation) false false))
    (:then_1
      (bind _returnvalue (UserInterface|CreateWidget "/Game/UI/WBP_HUD.WBP_HUD_C"))
      (bind _output_get (Variables|Default|SetWBP_HUD _returnvalue))
      (Default|InitHeartPiece (Variables|/Game/UI/WBP_HUD.WBP_HUD_C|GetWBP_HealthBox _output_get) (Variables|/Game/Blueprints/Components/HealthComponent.HealthComponent_C|GetMaxHealth (Variables|Default|GetHealthComponent)))
      (UserInterface|Viewport|AddtoViewport (Variables|Default|GetWBP_HUD) 0))))

(event EventHandleHitStates
  (|CallParentFunction)
  (Default|UpdateCurrentHealth (Variables|/Game/UI/WBP_HUD.WBP_HUD_C|GetWBP_HealthBox (Variables|Default|GetWBP_HUD)) (Variables|/Game/Blueprints/Components/HealthComponent.HealthComponent_C|GetCurrentHealth (Variables|Default|GetHealthComponent)))
  (Default|CallSetInvincibility (Variables|Default|GetHealthComponent))
  (|PlayAnimationOverridewithCallbacks (Variables|Default|GetAnimInstance) (Variables|Default|GetGetHitAnim) "DefaultSlot" 1.0 0.0
    (:then
      (Variables|Default|SetIsStunned true))
    (:OnCompleted
      (Variables|Default|SetIsStunned false :!label _label)
      (if (not (Default|IsAlive (Variables|Default|GetHealthComponent)))
        (Class|PaperZDAnimInstance|JumptoNode (Variables|Default|GetAnimInstance) "DeadJump" "None")
        (Utilities|FlowControl|Delay 2.0)
        (bind _returnvalue (Game|GetCurrentLevelName true))
        (Game|OpenLevel(byName) (Utilities|String|StringToName _returnvalue))
        (else
          (bind _returnvalue_2 (Utilities|Time|SetTimerbyEvent (EventDispatchers|CreateEvent :!event ToggleSpriteVisibility) (Variables|Default|GetSpriteFlickerInterval) true))
          (Variables|Default|SetSpriteFlickerTimer _returnvalue_2))))
    (:OnCancelled
      (goto _label))))

(fn ConstructionScript
  (|CallParentFunction))

(fn CanAct
  (return (Math|Boolean|ANDBoolean (not (Variables|Default|GetIsStunned)) (Default|IsAlive (Variables|Default|GetHealthComponent)) (not (Variables|Default|GetIsAttacking)))))

(fn SwordAttack
  (bind _arrayelement (Utilities|Array|ReverseforEachLoop (Collision|GetOverlappingActors (Variables|Default|GetHitBox) "/Game/Blueprints/Characters/BP_EnemyBase.BP_EnemyBase_C" :!class /Script/Engine.PrimitiveComponent))
    (:LoopBody
      (Game|Damage|ApplyDamage _arrayelement (Variables|Default|GetSwordDamage) 0 self))))

(fn FireArrow
  (bind _arrowpos (Variables|Default|GetArrowPos))
  (bind _returnvalue (Transformation|GetWorldTransform _arrowpos))
  (Game|SpawnActorfromClass "/Game/Blueprints/Projectiles/BP_Arrow.BP_Arrow_C" (Math|Transform|MakeTransform (.location _returnvalue) (.rotation _returnvalue) "1.000000,1.000000,1.000000") "AlwaysSpawn" "MultiplyWithRoot" self 0))

(fn GetHealed
  (params (HealAmount :type Float%20%28double-precision%29))
  (bind _healthcomponent (Variables|Default|GetHealthComponent))
  (Default|IncreaseHealth _healthcomponent HealAmount)
  (Default|UpdateCurrentHealth (Variables|/Game/UI/WBP_HUD.WBP_HUD_C|GetWBP_HealthBox (Variables|Default|GetWBP_HUD)) (Variables|/Game/Blueprints/Components/HealthComponent.HealthComponent_C|GetCurrentHealth _healthcomponent)))