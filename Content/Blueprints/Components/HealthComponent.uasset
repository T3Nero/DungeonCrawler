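; Health component that tracks an owner's current health, death state and damageability.
; Current health starts at the maximum on BeginPlay, and DecreaseHealth subtracts damage, clamps at zero and updates the dead flag.
; IsAlive and CanBeDamaged expose state to callers, the latter also honoring an invincibility flag.
; DecreaseHealth does not check invincibility itself and fires no death event.
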(event EventBeginPlay
  (Variables|Default|SetCurrentHealth (Variables|Default|GetMaxHealth)))

(event EventTick
  (params (DeltaSeconds :type Float%20%28single-precision%29)))

(fn DecreaseHealth
  (params (Damage :type Float%20%28double-precision%29))
  (Variables|Default|SetCurrentHealth (Math|Float|Max(Float) (- (Variables|Default|GetCurrentHealth) Damage) 0.0))
  (Variables|Default|SetIsDead (<= (Variables|Default|GetCurrentHealth) 0.0))
  (return))

(fn IsAlive
  (return (not (Variables|Default|GetIsDead))))

(fn CanbeDamaged
  (return (and (not (Variables|Default|GetIsDead)) (not (Variables|Default|GetIsInvincible)))))