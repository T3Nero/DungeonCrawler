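; Heart pickup item that restores health to the player who collects it.
; It overrides the parent's HandlePickUp event and, after calling it, acts only if the player's health is below maximum.
; It then heals by HealAmount, plays a 2D pickup sound and destroys itself, so it stays in place when health is full.
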(event EventBeginPlay
  (|CallParentFunction) ; This node is disabled and will not be called.\nDrag off pins to build functionality.
)

(event Collision|EventActorBeginOverlap
  (params (OtherActor :type Actor%20Object%20Reference))
  (|CallParentFunction OtherActor) ; This node is disabled and will not be called.\nDrag off pins to build functionality.
)

(event EventTick
  (params (DeltaSeconds :type Float%20%28single-precision%29))
  (|CallParentFunction DeltaSeconds) ; This node is disabled and will not be called.\nDrag off pins to build functionality.
)

(event EventHandlePickUp
  (params (Player :type BP%20Player%20Character%20Object%20Reference))
  (bind _healthcomponent (Variables|/Game/Blueprints/Characters/BP_BaseCharacter.BP_BaseCharacter_C|GetHealthComponent Player))
  (|CallParentFunction Player)
  (if (< (Variables|/Game/Blueprints/Components/HealthComponent.HealthComponent_C|GetCurrentHealth _healthcomponent) (Variables|/Game/Blueprints/Components/HealthComponent.HealthComponent_C|GetMaxHealth _healthcomponent))
    (Default|GetHealed Player (Variables|Default|GetHeal%20Amount))
    (Audio|PlaySound2D "/Game/Sounds/S_Pickup_Cue.S_Pickup_Cue" 1.0 1.0 0.0 0 0)
    (Actor|DestroyActor)))

(fn ConstructionScript
  (|CallParentFunction))